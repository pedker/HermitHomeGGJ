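; DecorationBP is a decoration actor that shows either a bubble particle effect or a rock mesh.
; The construction script checks IsParticle to assign the Bubbles template or a mesh picked at random from the first two Rocks entries, clearing the other component.
; The random pick is unseeded, and the event graph holds only disabled placeholder events, so there is no gameplay logic.
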(fn `UserConstructionScript`
  (if (`self.bIsParticle`)
    (`ParticleSystemComponent.SetTemplate` (`self.ParticleSystem`) "/Game/Particles/Bubbles.Bubbles")
    (`StaticMeshComponent.SetStaticMesh` (`self.StaticMesh`) null)
    (else
      (`ParticleSystemComponent.SetTemplate` (`self.ParticleSystem`) null)
      (`StaticMeshComponent.SetStaticMesh` (`self.StaticMesh`) (`|GetArrayItem` (`self.Rocks`) (`KismetMathLibrary.RandomIntegerInRange` 0 1))))))