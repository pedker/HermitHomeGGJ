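; TestChar is a test player character that moves on the yaw plane, can wear shells and grows by eating food.
; Functions attach collectibles to open shell sockets, flagging the shell full when none remain, and clear shell state on dropping.
; Eating enlarges the actor and resets attached actors' scale to one.
; Pickup, drop-message and hide logic is disconnected, while the shell upgrade and FoodMax check are empty stubs.
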(event `InputAxis|Forward`
  (params (AxisValue :type "Float (single-precision)"))
  (`self.AddMovementInput` (`KismetMathLibrary.GetForwardVector` (`KismetMathLibrary.MakeRotator` 0.0 0.0 (.yaw (`self.GetControlRotation`)))) AxisValue))

(event `InputAxis|Right`
  (params (AxisValue :type "Float (single-precision)"))
  (`self.AddMovementInput` (`KismetMathLibrary.GetRightVector` (`KismetMathLibrary.MakeRotator` 0.0 0.0 (.yaw (`self.GetControlRotation`)))) AxisValue))

(event `InputAction|Dropshell`
  (params (Key :type "Key Structure")))

(event `self.CapsuleComponent.OnComponentBeginOverlap`
  (params (OverlappedComponent :type "PrimitiveComponent Object Reference") (OtherActor :type "Actor Object Reference") (OtherComp :type "PrimitiveComponent Object Reference") (OtherBodyIndex :type Integer) (bFromSweep :type Boolean) (SweepResult :type "HitResult Structure (by ref)")))

(event `self.ReceiveTick`
  (params (DeltaSeconds :type "Float (single-precision)")))

(fn `AttachCollectible`
  (if (== (`KismetArrayLibrary.Array_Length` (`self.OpenSockets`)) 0)
    (set `/Game/Blueprints/Shell/ShellBP.bIsFull` true (`self.CurrentShell`))
    (else
      (`self.K2_AttachToComponent` (`self.Collectible`) (`/Game/Blueprints/Shell/ShellBP.StaticMesh` (`self.CurrentShell`)) (`|GetArrayItem` (`self.OpenSockets`)) "SnapToTarget" "SnapToTarget" "KeepWorld" true)
      (`KismetArrayLibrary.Array_Remove` (`self.OpenSockets`))
      (set `/Game/Blueprints/CollectableBP.bIsAttached` true (`self.Collectible`)))))

(fn `DroppingShell`
  (set `self.CurrentShell` null)
  (set `self.hasShell` false)
  (set `self.isHidden` false))

(fn `IncreaseFood`
  (bind _currentshell (`self.CurrentShell`))
  (bind (_shell_weight _shell_shellmesh _shell_foodmin _shell_foodmax) (break `/Game/Blueprints/Shell/ShellStruct` (`/Game/Blueprints/Shell/ShellBP.Shell` _currentshell)))
  (bind _result (`/Engine/EditorBlueprintResources/StandardMacros.IncrementInt` (`self.Food`))
    (:`  `
      (`self.SetActorScale3D` (+ (`self.GetActorScale3D`) (0.2 0.2 0.2)))
      (for _array_element (`self.GetAttachedActors`)
        (`self.SetActorScale3D` _array_element (1.0 1.0 1.0)))
      (`/Engine/EditorBlueprintResources/StandardMacros.IsValid` _currentshell
        (:`Is Valid`
          (if (> _result _shell_foodmax)
            _))))))

(fn `ShouldUpgradeShell`)

(fn `UserConstructionScript`)