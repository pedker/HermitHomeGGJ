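; Player controller Blueprint that runs the death and game-over sequence for the TopDownCharacter.
; EndGameScreen fires once, only if the character can be damaged, then destroys the pawn and possesses a SpectatorPawn spawned at its camera transform.
; It shows the GameOver widget while a timeline lerps the spectator straight up from the camera position for a pull-away shot.
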(event `EndGameScreen`
  (bind _returnvalue (`self.K2_GetPawn`))
  (bind _cameratransform_location (`KismetMathLibrary.BreakTransform` (`self.CameraTransform`)))
  (bind _astop_down_character (cast `/Game/Blueprints/TopDownCharacter` (`self.K2_GetPawn` (`GameplayStatics.GetPlayerController` 0))))
  (if (`Actor.bCanBeDamaged` _astop_down_character)
    (if (not (`self.bIsDead`))
      (set `self.bIsDead` true)
      (bind _astop_down_character_2 (cast `/Game/Blueprints/TopDownCharacter` _returnvalue))
      (set `self.CameraTransform` (`SceneComponent.K2_GetComponentToWorld` (`/Game/Blueprints/TopDownCharacter.Camera1` _astop_down_character_2)))
      (set `self.food` (`/Game/Blueprints/TopDownCharacter.Food` _astop_down_character_2))
      (`self.K2_DestroyActor` _returnvalue)
      (bind _returnvalue_2 (`|SpawnActorFromClass` "/Game/Blueprints/SpectatorPawn.SpectatorPawn_C" (`self.CameraTransform`) "AlwaysSpawn" "OverrideRootScale" null null))
      (`self.Possess` _returnvalue_2)
      (bind _returnvalue_3 (`|CreateWidget` "/Game/Blueprints/UI/GameOver.GameOver_C" self))
      (`UserWidget.AddToViewport` _returnvalue_3 0)
      (bind (_direction _newtrack_0) (`Timeline|Timeline_0` :!via `PlayFromStart`)
        (:`Update`
          (`self.K2_SetActorLocation` _returnvalue_2 (`KismetMathLibrary.VLerp` _cameratransform_location (+ _cameratransform_location (0.0 0.0 10000.0)) _newtrack_0) false false))))))

(fn `UserConstructionScript`)