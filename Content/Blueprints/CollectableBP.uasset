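; Collectable actor that attaches itself to the player's current shell when picked up.
; Pickup runs only with a valid, non-full shell and while the item is unattached.
; It snaps to the first of the player's open sockets on the shell mesh, keeping world scale, then removes that socket and marks itself attached.
; If no open sockets remain, it flags the shell as full instead.
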(event `/Game/Blueprints/PickupInterface.Pickup`
  (params (Player :type "/Game/Blueprints/TopDownCharacter Object Reference"))
  (bind _currentshell (`/Game/Blueprints/TopDownCharacter.CurrentShell` Player))
  (bind _currentshell_2 (`/Game/Blueprints/TopDownCharacter.CurrentShell` Player))
  (`/Engine/EditorBlueprintResources/StandardMacros.IsValid` _currentshell
    (:`Is Valid`
      (if (`self.bIsAttached`)
        _
        (elif (`/Game/Blueprints/Shell/ShellBP.bIsFull` _currentshell)
          _
          (elif (== (`KismetArrayLibrary.Array_Length` (`/Game/Blueprints/TopDownCharacter.OpenSockets` Player)) 0)
            (set `/Game/Blueprints/Shell/ShellBP.bIsFull` true _currentshell_2)
            (else
              (`self.K2_AttachToComponent` self (`/Game/Blueprints/Shell/ShellBP.StaticMesh` _currentshell_2) (`|GetArrayItem` (`/Game/Blueprints/TopDownCharacter.OpenSockets` Player)) "SnapToTarget" "SnapToTarget" "KeepWorld" true)
              (`KismetArrayLibrary.Array_Remove` (`/Game/Blueprints/TopDownCharacter.OpenSockets` Player))
              (set `self.bIsAttached` true))))))))

(fn `UserConstructionScript`)