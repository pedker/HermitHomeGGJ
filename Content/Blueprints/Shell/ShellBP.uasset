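; Shell actor that the player can wear on their head and drop, with its data and mesh chosen by tier at construction.
; Pickup requires a shell-less player with Food in the tier's range, then attaches to the head socket and hands the mesh's socket names to the player.
; Drop detaches it, snaps it to the ground with a downward trace and notifies the player.
; A used flag makes each shell a one-time pickup.
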(event `/Game/Blueprints/PickupInterface.Drop`
  (params (Player :type "/Game/Blueprints/TopDownCharacter Object Reference"))
  (`self.K2_DetachFromActor` "KeepWorld" "KeepWorld" "KeepWorld")
  (`self.DropToGround`)
  (set `self.bHasBeenUsed` true)
  (`/Game/Blueprints/TopDownCharacter.DroppingShell` Player))

(event `/Game/Blueprints/PickupInterface.Pickup`
  (params (Player :type "/Game/Blueprints/TopDownCharacter Object Reference"))
  (bind _food (`/Game/Blueprints/TopDownCharacter.Food` Player))
  (bind (_shell_weight _shell_shellmesh _shell_foodmin _shell_foodmax) (break `/Game/Blueprints/Shell/ShellStruct` (`self.Shell`)))
  (if (`/Game/Blueprints/TopDownCharacter.hasShell` Player)
    _
    (elif (`self.bHasBeenUsed`)
      _
      (elif (and (>= _food _shell_foodmin) (<= _food _shell_foodmax))
        (`self.K2_AttachToComponent` self (`Character.Mesh` Player) "headSocket" "SnapToTarget" "KeepRelative" "KeepWorld" true)
        (set `/Game/Blueprints/TopDownCharacter.CurrentShell` self Player)
        (set `/Game/Blueprints/TopDownCharacter.OpenSockets` (`SceneComponent.GetAllSocketNames` (`self.StaticMesh`)) Player)
        (set `self.bHasBeenUsed` true)
        (set `/Game/Blueprints/TopDownCharacter.hasShell` true Player)))))

(fn `DropToGround`
  (bind _returnvalue (`self.K2_GetActorLocation`))
  (bind _outhit (`KismetSystemLibrary.LineTraceSingle` _returnvalue (- _returnvalue (0.0 0.0 100000.0)) "TraceTypeQuery1"))
  (`self.K2_SetActorLocation` (`.ImpactPoint` (`GameplayStatics.BreakHitResult` _outhit))))

(fn `UserConstructionScript`
  (bind _output_get (set `self.Shell` (`|GetArrayItem` (`self.ShellTierArray`) (`self.ShellTier`))))
  (`StaticMeshComponent.SetStaticMesh` (`self.StaticMesh`) (`.ShellMesh_9_F92976B94F0A0A37250C17B622D0FB3D` (break `/Game/Blueprints/Shell/ShellStruct` _output_get))))