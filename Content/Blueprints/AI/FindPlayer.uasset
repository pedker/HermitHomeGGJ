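; FindPlayer is a behavior tree node that updates the Player blackboard key on each AI tick.
; It clears the key when the controlled pawn's location equals the player pawn's within a 500-unit tolerance.
; Otherwise it casts the player pawn to TopDownCharacter, clearing the key if IsHidden is true and storing the pawn if not.
; A failed cast leaves the key unchanged.
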(event `self.ReceiveTickAI`
  (params (OwnerController :type "AIController Object Reference") (ControlledPawn :type "Pawn Object Reference") (DeltaSeconds :type "Float (single-precision)"))
  (bind _returnvalue (`Controller.K2_GetPawn` (`GameplayStatics.GetPlayerController` 0)))
  (if (== (`Actor.K2_GetActorLocation` ControlledPawn) (`Actor.K2_GetActorLocation` _returnvalue) :`ErrorTolerance` 500.0)
    (`BTFunctionLibrary.SetBlackboardValueAsObject` (`self.Player`) :!label _label)
    (else
      (bind _astop_down_character (cast `/Game/Blueprints/TopDownCharacter` _returnvalue))
      (if (`/Game/Blueprints/TopDownCharacter.isHidden` _astop_down_character)
        (goto _label)
        (else
          (`BTFunctionLibrary.SetBlackboardValueAsObject` (`self.Player`) _returnvalue))))))