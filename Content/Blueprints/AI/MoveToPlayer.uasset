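; Behavior tree task that sends an AI pawn after the player-controlled TopDownCharacter.
; If the player is hidden, it clears the Player blackboard key and finishes successfully.
; Otherwise it uses AIMoveTo toward the player, and on arrival calls DropMessage on the player's CurrentShell before finishing.
; A failed move or failed cast never calls FinishExecute.
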(event `self.ReceiveTickAI`
  (params (OwnerController :type "AIController Object Reference") (ControlledPawn :type "Pawn Object Reference") (DeltaSeconds :type "Float (single-precision)"))
  (bind _returnvalue (`Controller.K2_GetPawn` (`GameplayStatics.GetPlayerController` 0)))
  (bind _astop_down_character (cast `/Game/Blueprints/TopDownCharacter` _returnvalue))
  (if (`/Game/Blueprints/TopDownCharacter.isHidden` _astop_down_character)
    (`BTFunctionLibrary.SetBlackboardValueAsObject` (`self.Player`))
    (`self.FinishExecute` true)
    (else
      (`|AIMoveTo` ControlledPawn (`Actor.K2_GetActorLocation` _returnvalue) _returnvalue 30.0
        (:`OnSuccess`
          (message `/Game/Blueprints/PickupInterface.Drop` (`/Game/Blueprints/TopDownCharacter.CurrentShell` _astop_down_character) _astop_down_character)
          (`self.FinishExecute` true))))))